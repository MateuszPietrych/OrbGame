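; GA_FireBall is a Gameplay Ability that launches a projectile, named as a fireball, through SpawnProjectile.
; Plain activation fires from the OrbUseContext source owner's location along the context's direction.
; Event activation casts the instigator to OrbGameCharacter and fires from its location toward the mouse, using its PlayerController.
; Both paths target a fixed distance along that direction and print debug strings; neither calls EndAbility here.
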(event Ability|EventActivateAbility
  (bind _orbusecontext (Variables|Default|GetOrbUseContext))
  (bind _returnvalue (Components|GetOwner (.sourceabilitysystemcomponent _orbusecontext)))
  (bind _returnvalue_2 (Transformation|GetActorLocation _returnvalue))
  (Development|PrintString "Hello 1")
  (Class|ProjectileGameplayAbility|SpawnProjectile (+ (* (.direction _orbusecontext) (Math|Conversions|ToVector(Float) 1e+03)) _returnvalue_2) _returnvalue_2)
  (Development|PrintString "Hello 2"))

(event Ability|EventOnEndAbility
  (params (bWasCancelled :type Boolean)))

(event Ability|EventActivateAbilityFromEvent
  (params (EventData :type Gameplay%20Event%20Data%20Structure%20%28by%20ref%29))
  (bind _instigator (Utilities|Struct|BreakGameplayEventData EventData))
  (bind _returnvalue (Transformation|GetActorLocation _instigator))
  (bind _asorb_game_character (Utilities|Casting|CastToOrbGameCharacter _instigator))
  (bind _asplayer_controller (Utilities|Casting|CastToPlayerController (Pawn|GetController _asorb_game_character)))
  (bind _returnvalue_2 (Class|OrbGameBlueprintLibrary|FromPlayertoMouseDirection _asplayer_controller))
  (Development|PrintString "Hello event 1")
  (Class|ProjectileGameplayAbility|SpawnProjectile (+ (* _returnvalue_2 (Math|Conversions|ToVector(Float) 1e+03)) _returnvalue) _returnvalue))